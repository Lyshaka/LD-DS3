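; BP_GiantDoor is a double door that swings open once all of its locks are unlocked.
; Its construction script gathers child BP_Lock actors and assigns each the lever at the matching index in its Levers array.
; Tick polls every lock, then fires a one-time timeline that rotates the left and right hinges in opposite yaw directions.
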(event `self.ReceiveTick`
  (params (DeltaSeconds :type "Float (single-precision)"))
  (bind _unlocked (`self.DoorUnlocked` (`self.Locks`)))
  (if _unlocked
    (`/Engine/EditorBlueprintResources/StandardMacros.DoOnce` false
      (:`Completed`
        (`self.OpenDoor`)))))

(event `OpenDoor`
  (bind (_direction _movement) (`Timeline|DoorMovement`)
    (:`Update`
      (`SceneComponent.K2_SetRelativeRotation` (`self.LeftHinge`) (`KismetMathLibrary.MakeRotator` 0.0 0.0 _movement) false false)
      (`SceneComponent.K2_SetRelativeRotation` (`self.RightHinge`) (`KismetMathLibrary.MakeRotator` 0.0 0.0 (* _movement -1.0)) false false))))

(fn `DoorUnlocked`
  (params (Locks :type "Array of Actor Object Reference"))
  (returns (Unlocked :type Boolean))
  (for _array_element Locks
    (bind _asbp_lock (cast `/Game/Actors/BP_Lock` _array_element))
    (if (not (`/Game/Actors/BP_Lock.Unlocked` _asbp_lock))
      (return false)))
  (return true))

(fn `UserConstructionScript`
  (bind _output_get (set `self.Locks` (`self.GetAllChildActors` true)))
  (for (_array_element _array_index) _output_get
    (bind _asbp_lock (cast `/Game/Actors/BP_Lock` _array_element))
    (set `/Game/Actors/BP_Lock.Lever` (`|GetArrayItem` (`self.Levers`) _array_index) _asbp_lock)))