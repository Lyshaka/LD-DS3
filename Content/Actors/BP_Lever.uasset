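; BP_Lever is a one-use lever that the player pulls with E while standing in its collision sphere.
; Overlap by a grounded, living BP_ThirdPersonCharacter sets Inside and tells the game mode interaction is available; leaving reverses both.
; Tick polls the key and, through a DoOnce, starts Activate, destroys the trigger and sets Activated.
; Activate plays a timeline that drives the pitch of the Sphere component.
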(event `self.ReceiveTick`
  (params (DeltaSeconds :type "Float (single-precision)"))
  (if (and (`PlayerController.IsInputKeyDown` (`GameplayStatics.GetPlayerController` 0) "E") (`self.Inside`))
    (`/Engine/EditorBlueprintResources/StandardMacros.DoOnce` false
      (:`Completed`
        (`self.Activate`)
        (`ActorComponent.K2_DestroyComponent` (`self.CollisionSphere`))
        (set `self.Activated` true)))))

(event `self.CollisionSphere.OnComponentBeginOverlap`
  (params (OverlappedComponent :type "PrimitiveComponent Object Reference") (OtherActor :type "Actor Object Reference") (OtherComp :type "PrimitiveComponent Object Reference") (OtherBodyIndex :type Integer) (bFromSweep :type Boolean) (SweepResult :type "HitResult Structure (by ref)"))
  (bind _asbp_third_person_character (cast `/Game/ThirdPerson/Blueprints/BP_ThirdPersonCharacter` OtherActor))
  (bind _gamemode (`/Game/ThirdPerson/Blueprints/BP_ThirdPersonCharacter.Gamemode` _asbp_third_person_character))
  (if (`KismetMathLibrary.BooleanNOR` (`NavMovementComponent.IsFalling` (`Character.CharacterMovement` _asbp_third_person_character)) (`/Game/ThirdPerson/Blueprints/BP_ThirdPersonGameMode.PlayerDead` _gamemode))
    (set `self.Inside` true)
    (`/Game/ThirdPerson/Blueprints/BP_ThirdPersonGameMode.CanInteract` _gamemode)))

(event `self.CollisionSphere.OnComponentEndOverlap`
  (params (OverlappedComponent :type "PrimitiveComponent Object Reference") (OtherActor :type "Actor Object Reference") (OtherComp :type "PrimitiveComponent Object Reference") (OtherBodyIndex :type Integer))
  (bind _asbp_third_person_character (cast `/Game/ThirdPerson/Blueprints/BP_ThirdPersonCharacter` OtherActor))
  (`/Game/ThirdPerson/Blueprints/BP_ThirdPersonGameMode.CannotInteract` (`/Game/ThirdPerson/Blueprints/BP_ThirdPersonCharacter.Gamemode` _asbp_third_person_character))
  (set `self.Inside` false))

(event `Activate`
  (bind (_direction _movement) (`Timeline|Timeline` :!via `PlayFromStart`)
    (:`Update`
      (`SceneComponent.K2_SetRelativeRotation` (`self.Sphere`) (`KismetMathLibrary.MakeRotator` 0.0 _movement) false false))))

(fn `UserConstructionScript`)