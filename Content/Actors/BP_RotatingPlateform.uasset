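; BP_RotatingPlateform is an actor that spins a configurable number of platform instances around the vertical axis.
; The Construction Script adds evenly yawed instanced meshes and scales the Rotation timeline's play rate from Speed.
; On BeginPlay the timeline plays forward, or in reverse when CounterClockwise is set.
; Its Degree track sets the world yaw of Pivot, while CounterPivot receives the opposite yaw.
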(event `self.ReceiveBeginPlay`
  (if (`self.CounterClockwise`)
    (bind (_direction _degree) (`Timeline|Rotation` :!via `Reverse` :!label _label)
      (:`Update`
        (`SceneComponent.K2_SetWorldRotation` (`self.Pivot`) (`KismetMathLibrary.MakeRotator` 0.0 0.0 _degree) false false)
        (`SceneComponent.K2_SetWorldRotation` (`self.CounterPivot`) (`KismetMathLibrary.MakeRotator` 0.0 0.0 (- 360.0 _degree)) false false)))
    (else
      (goto _label))))

(fn `UserConstructionScript`
  (`|ExecutionSequence`
    (:`then_0`
      (`TimelineComponent.SetPlayRate` (`self.Rotation`) (/ (`self.Speed`) 100.0)))
    (:`then_1`
      (for _index (range 1 (+ (`self.NbPlateform`) 1))
        (`InstancedStaticMeshComponent.AddInstance` (`self.Plateform`) (`KismetMathLibrary.MakeTransform` (0.0 0.0 0.0) (`KismetMathLibrary.MakeRotator` 0.0 90.0 (* _index (/ 360 (`self.NbPlateform`))))) false)))))