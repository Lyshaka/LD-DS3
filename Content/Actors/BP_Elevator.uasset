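; Elevator actor that carries the player between a bottom and top stop, with configurable height, speed and starting position.
; Trigger boxes at each lever enable polling for the E key on Tick, which animates the lever and calls the elevator to that end.
; Overlapping the elevator's box moves a slab and starts a timer that sends it to the opposite end.
; A single timeline drives travel, its play rate scaled by Speed over Height.
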(event `self.ReceiveTick`
  (params (DeltaSeconds :type "Float (single-precision)"))
  (`|ExecutionSequence`
    (:`then_0`
      (if (`self.NearTopLever`)
        (if (`PlayerController.IsInputKeyDown` (`GameplayStatics.GetPlayerController` 0) "E")
          (`/Engine/EditorBlueprintResources/StandardMacros.DoOnce` false :!label _label
            (:`Completed`
              (`self.ActivateLever` (`self.TopLever`))
              (`|ExecutionSequence`
                (:`then_0`
                  (`self.GoUp`))
                (:`then_1`
                  (`KismetSystemLibrary.Delay` 1.0)
                  (goto _label :!via `Reset`))))))))
    (:`then_1`
      (if (`self.NearBottomLever`)
        (if (`PlayerController.IsInputKeyDown` (`GameplayStatics.GetPlayerController` 0) "E")
          (`/Engine/EditorBlueprintResources/StandardMacros.DoOnce` false :!label _label_2
            (:`Completed`
              (`self.ActivateLever` (`self.BottomLever`))
              (`|ExecutionSequence`
                (:`then_0`
                  (`self.GoDown`))
                (:`then_1`
                  (`KismetSystemLibrary.Delay` 1.0)
                  (goto _label_2 :!via `Reset`))))))))))

(event `self.TopBox.OnComponentBeginOverlap`
  (params (OverlappedComponent :type "PrimitiveComponent Object Reference") (OtherActor :type "Actor Object Reference") (OtherComp :type "PrimitiveComponent Object Reference") (OtherBodyIndex :type Integer) (bFromSweep :type Boolean) (SweepResult :type "HitResult Structure (by ref)"))
  (bind _asbp_third_person_character (cast `/Game/ThirdPerson/Blueprints/BP_ThirdPersonCharacter` OtherActor))
  (bind _gamemode (`/Game/ThirdPerson/Blueprints/BP_ThirdPersonCharacter.Gamemode` _asbp_third_person_character))
  (if (`KismetMathLibrary.BooleanNOR` (`NavMovementComponent.IsFalling` (`Character.CharacterMovement` _asbp_third_person_character)) (`/Game/ThirdPerson/Blueprints/BP_ThirdPersonGameMode.PlayerDead` _gamemode))
    (set `self.NearTopLever` true)
    (`/Game/ThirdPerson/Blueprints/BP_ThirdPersonGameMode.CanInteract` _gamemode)))

(event `self.TopBox.OnComponentEndOverlap`
  (params (OverlappedComponent :type "PrimitiveComponent Object Reference") (OtherActor :type "Actor Object Reference") (OtherComp :type "PrimitiveComponent Object Reference") (OtherBodyIndex :type Integer))
  (bind _asbp_third_person_character (cast `/Game/ThirdPerson/Blueprints/BP_ThirdPersonCharacter` OtherActor))
  (`/Game/ThirdPerson/Blueprints/BP_ThirdPersonGameMode.CannotInteract` (`/Game/ThirdPerson/Blueprints/BP_ThirdPersonCharacter.Gamemode` _asbp_third_person_character))
  (set `self.NearTopLever` false))

(event `self.BottomBox.OnComponentBeginOverlap`
  (params (OverlappedComponent :type "PrimitiveComponent Object Reference") (OtherActor :type "Actor Object Reference") (OtherComp :type "PrimitiveComponent Object Reference") (OtherBodyIndex :type Integer) (bFromSweep :type Boolean) (SweepResult :type "HitResult Structure (by ref)"))
  (bind _asbp_third_person_character (cast `/Game/ThirdPerson/Blueprints/BP_ThirdPersonCharacter` OtherActor))
  (bind _gamemode (`/Game/ThirdPerson/Blueprints/BP_ThirdPersonCharacter.Gamemode` _asbp_third_person_character))
  (if (`KismetMathLibrary.BooleanNOR` (`NavMovementComponent.IsFalling` (`Character.CharacterMovement` _asbp_third_person_character)) (`/Game/ThirdPerson/Blueprints/BP_ThirdPersonGameMode.PlayerDead` _gamemode))
    (set `self.NearBottomLever` true)
    (`/Game/ThirdPerson/Blueprints/BP_ThirdPersonGameMode.CanInteract` _gamemode)))

(event `self.BottomBox.OnComponentEndOverlap`
  (params (OverlappedComponent :type "PrimitiveComponent Object Reference") (OtherActor :type "Actor Object Reference") (OtherComp :type "PrimitiveComponent Object Reference") (OtherBodyIndex :type Integer))
  (bind _asbp_third_person_character (cast `/Game/ThirdPerson/Blueprints/BP_ThirdPersonCharacter` OtherActor))
  (`/Game/ThirdPerson/Blueprints/BP_ThirdPersonGameMode.CannotInteract` (`/Game/ThirdPerson/Blueprints/BP_ThirdPersonCharacter.Gamemode` _asbp_third_person_character))
  (set `self.NearBottomLever` false))

(event `ActivateLever`
  (params (Lever :type "SceneComponent Object Reference"))
  (bind (_direction _movement) (`Timeline|LeverMovement` :!via `PlayFromStart`)
    (:`Update`
      (`SceneComponent.K2_SetRelativeRotation` Lever (`KismetMathLibrary.MakeRotator` 0.0 _movement) false false))))

(event `GoUp`
  (bind (_direction _movement) (`Timeline|ElevatorMovement` :!label _label_3)
    (:`Update`
      (set `self.Progression` _movement)
      (`SceneComponent.K2_SetRelativeLocation` (`self.Elevator`) (`KismetMathLibrary.MakeVector` 0.0 0.0 (+ (* _movement (`self.Height`)) 100.0)) false false))))

(event `GoDown`
  (goto _label_3 :!via `Reverse`))

(event `self.ElevatorBox.OnComponentBeginOverlap`
  (params (OverlappedComponent :type "PrimitiveComponent Object Reference") (OtherActor :type "Actor Object Reference") (OtherComp :type "PrimitiveComponent Object Reference") (OtherBodyIndex :type Integer) (bFromSweep :type Boolean) (SweepResult :type "HitResult Structure (by ref)"))
  (`|ExecutionSequence`
    (:`then_0`
      (bind (_direction _movement) (`Timeline|SlabMovement` :!label _label_4)
        (:`Update`
          (`SceneComponent.K2_SetRelativeLocation` (`self.Slab`) (`KismetMathLibrary.MakeVector` 0.0 0.0 _movement) false false))))
    (:`then_1`
      (`/Engine/EditorBlueprintResources/StandardMacros.DoOnce` false :!label _label_5
        (:`Completed`
          (`Timeline|Timer` :!via `PlayFromStart` :!label _label_6
            (:`Finished`
              (`self.ActivateElevator`))))))))

(event `self.ElevatorBox.OnComponentEndOverlap`
  (params (OverlappedComponent :type "PrimitiveComponent Object Reference") (OtherActor :type "Actor Object Reference") (OtherComp :type "PrimitiveComponent Object Reference") (OtherBodyIndex :type Integer))
  (`|ExecutionSequence`
    (:`then_0`
      (goto _label_4 :!via `Reverse`))
    (:`then_1`
      (goto _label_6 :!via `Stop`))
    (:`then_2`
      (goto _label_5 :!via `Reset`))))

(event `ActivateElevator`
  (`|ExecutionSequence`
    (:`then_0`
      (if (== (`self.Progression`) 1.0)
        (`self.GoDown`)))
    (:`then_1`
      (if (== (`self.Progression`) 0.0)
        (`self.GoUp`)))))

(fn `UserConstructionScript`
  (`SceneComponent.K2_SetRelativeLocation` (`self.SM_ElevatorShaft_Top`) (`KismetMathLibrary.MakeVector` 0.0 0.0 (`self.Height`)) false false)
  (`TimelineComponent.SetPlayRate` (`self.ElevatorMovement`) (/ (`self.Speed`) (`self.Height`)))
  (if (`self.IsElevatorUp`)
    (set `self.Progression` 1.0)
    (`SceneComponent.K2_SetRelativeLocation` (`self.Elevator`) (`KismetMathLibrary.MakeVector` 0.0 0.0 (+ (`self.Height`) 100.0)) false false)
    (`TimelineComponent.SetNewTime` (`self.ElevatorMovement`) 1.0)))