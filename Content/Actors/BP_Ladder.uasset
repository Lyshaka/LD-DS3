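; BP_Ladder is a ladder that teleports the player between its top and bottom, optionally starting closed until opened from the top.
; The construction script builds instanced segments from LadderHeight and positions the Top trigger, leaving only the highest segment when closed.
; Top and Bottom overlaps set proximity flags and notify the Gamemode of interactability.
; Tick polls E through a DoOnce to teleport, or to unfold a closed ladder by adding the missing segments.
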(event `self.ReceiveBeginPlay`
  (if (`self.IsClosed`)
    (`ActorComponent.Deactivate` (`self.Bottom`))))

(event `self.Top.OnComponentBeginOverlap`
  (params (OverlappedComponent :type "PrimitiveComponent Object Reference") (OtherActor :type "Actor Object Reference") (OtherComp :type "PrimitiveComponent Object Reference") (OtherBodyIndex :type Integer) (bFromSweep :type Boolean) (SweepResult :type "HitResult Structure (by ref)"))
  (bind _asbp_third_person_character (cast `/Game/ThirdPerson/Blueprints/BP_ThirdPersonCharacter` OtherActor))
  (bind _gamemode (`/Game/ThirdPerson/Blueprints/BP_ThirdPersonCharacter.Gamemode` _asbp_third_person_character))
  (`/Engine/EditorBlueprintResources/StandardMacros.IsValid` _gamemode
    (:`Is Valid`
      (if (`KismetMathLibrary.BooleanNOR` (`NavMovementComponent.IsFalling` (`Character.CharacterMovement` _asbp_third_person_character)) (`/Game/ThirdPerson/Blueprints/BP_ThirdPersonGameMode.PlayerDead` _gamemode))
        (set `self.NearTop` true)
        (`/Game/ThirdPerson/Blueprints/BP_ThirdPersonGameMode.CanInteract` _gamemode)))))

(event `self.Top.OnComponentEndOverlap`
  (params (OverlappedComponent :type "PrimitiveComponent Object Reference") (OtherActor :type "Actor Object Reference") (OtherComp :type "PrimitiveComponent Object Reference") (OtherBodyIndex :type Integer))
  (bind _asbp_third_person_character (cast `/Game/ThirdPerson/Blueprints/BP_ThirdPersonCharacter` OtherActor))
  (`/Game/ThirdPerson/Blueprints/BP_ThirdPersonGameMode.CannotInteract` (`/Game/ThirdPerson/Blueprints/BP_ThirdPersonCharacter.Gamemode` _asbp_third_person_character))
  (set `self.NearTop` false))

(event `self.Bottom.OnComponentBeginOverlap`
  (params (OverlappedComponent :type "PrimitiveComponent Object Reference") (OtherActor :type "Actor Object Reference") (OtherComp :type "PrimitiveComponent Object Reference") (OtherBodyIndex :type Integer) (bFromSweep :type Boolean) (SweepResult :type "HitResult Structure (by ref)"))
  (bind _asbp_third_person_character (cast `/Game/ThirdPerson/Blueprints/BP_ThirdPersonCharacter` OtherActor))
  (bind _gamemode (`/Game/ThirdPerson/Blueprints/BP_ThirdPersonCharacter.Gamemode` _asbp_third_person_character))
  (`/Engine/EditorBlueprintResources/StandardMacros.IsValid` _gamemode
    (:`Is Valid`
      (if (`KismetMathLibrary.BooleanNOR` (`NavMovementComponent.IsFalling` (`Character.CharacterMovement` _asbp_third_person_character)) (`/Game/ThirdPerson/Blueprints/BP_ThirdPersonGameMode.PlayerDead` _gamemode))
        (if (not (`self.IsClosed`))
          (set `self.NearBottom` true)
          (`/Game/ThirdPerson/Blueprints/BP_ThirdPersonGameMode.CanInteract` _gamemode))))))

(event `self.Bottom.OnComponentEndOverlap`
  (params (OverlappedComponent :type "PrimitiveComponent Object Reference") (OtherActor :type "Actor Object Reference") (OtherComp :type "PrimitiveComponent Object Reference") (OtherBodyIndex :type Integer))
  (bind _asbp_third_person_character (cast `/Game/ThirdPerson/Blueprints/BP_ThirdPersonCharacter` OtherActor))
  (`/Game/ThirdPerson/Blueprints/BP_ThirdPersonGameMode.CannotInteract` (`/Game/ThirdPerson/Blueprints/BP_ThirdPersonCharacter.Gamemode` _asbp_third_person_character))
  (set `self.NearBottom` false))

(event `self.ReceiveTick`
  (params (DeltaSeconds :type "Float (single-precision)"))
  (if (or (`self.NearBottom`) (`self.NearTop`))
    (if (`PlayerController.IsInputKeyDown` (`GameplayStatics.GetPlayerController` 0) "E")
      (`/Engine/EditorBlueprintResources/StandardMacros.DoOnce` false :!label _label
        (:`Completed`
          (if (`self.NearTop`)
            (if (not (`self.IsClosed`))
              (`self.K2_TeleportTo` (`GameplayStatics.GetPlayerPawn` 0) (+ (`SceneComponent.K2_GetComponentLocation` (`self.Bottom`)) (0.0 0.0 50.0)) (`CharacterMovementComponent.GetLastUpdateRotation` (`Character.CharacterMovement` (`GameplayStatics.GetPlayerCharacter` 0))))
              (else
                (`self.ActivateLadder`)))
            (else
              (`self.K2_TeleportTo` (`GameplayStatics.GetPlayerPawn` 0) (+ (`SceneComponent.K2_GetComponentLocation` (`self.Top`)) (0.0 0.0 50.0)) (`CharacterMovementComponent.GetLastUpdateRotation` (`Character.CharacterMovement` (`GameplayStatics.GetPlayerCharacter` 0))))))))
      (else
        (goto _label :!via `Reset`)))))

(event `ActivateLadder`
  (`ActorComponent.Activate` (`self.Bottom`) true)
  (set `self.IsClosed` false)
  (for _index (range 1 (`self.LadderHeight`))
    (`InstancedStaticMeshComponent.AddInstance` (`self.Ladder`) (`KismetMathLibrary.MakeTransform` (`KismetMathLibrary.MakeVector` 0.0 10.0 (- (* _index 100.0) 50.0))) false)))

(fn `UserConstructionScript`
  (if (not (`self.IsClosed`))
    (for _index (range 1 (+ (`self.LadderHeight`) 1))
      (bind _returnvalue (`InstancedStaticMeshComponent.AddInstance` (`self.Ladder`) (`KismetMathLibrary.MakeTransform` (`KismetMathLibrary.MakeVector` 0.0 10.0 (- (* _index 100.0) 50.0))) false))
      (`SceneComponent.K2_SetRelativeLocation` (`self.Top`) (`KismetMathLibrary.MakeVector` 0.0 -100.0 (+ (* _returnvalue 100.0) 200.0)) false false))
    (else
      (`InstancedStaticMeshComponent.AddInstance` (`self.Ladder`) (`KismetMathLibrary.MakeTransform` (`KismetMathLibrary.MakeVector` 0.0 10.0 (- (* (`self.LadderHeight`) 100.0) 50.0))) false)
      (`SceneComponent.K2_SetRelativeLocation` (`self.Top`) (`KismetMathLibrary.MakeVector` 0.0 -100.0 (+ (* (`self.LadderHeight`) 100.0) 100.0)) false false))))