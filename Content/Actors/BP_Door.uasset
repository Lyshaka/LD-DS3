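; BP_Door is an interactable door that can require a key or open only from permitted sides.
; Front and Back overlaps track whether a grounded, living player is in range and on a valid side, toggling the game mode's interact prompt.
; Tick polls the E key, then either shows a refusal message or plays a timeline rotating the door and destroys both triggers.
; The construction script colour-codes side labels by access rule and sets helper component visibility.
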(event `self.ReceiveBeginPlay`
  (bind _returnvalue (`GameplayStatics.GetActorOfClass` "/Game/ThirdPerson/Blueprints/BP_ThirdPersonGameMode.BP_ThirdPersonGameMode_C"))
  (set `self.Gamemode` _returnvalue))

(event `self.ReceiveTick`
  (params (DeltaSeconds :type "Float (single-precision)"))
  (if (`self.Inside`)
    (if (`PlayerController.IsInputKeyDown` (`GameplayStatics.GetPlayerController` 0) "E")
      (if (`self.RequireKey`)
        (bind _asbp_third_person_character (cast `/Game/ThirdPerson/Blueprints/BP_ThirdPersonCharacter` (`GameplayStatics.GetPlayerCharacter` 0)))
        (if (`/Game/ThirdPerson/Blueprints/BP_ThirdPersonCharacter.PlayerHasKey` _asbp_third_person_character (`self.Key`))
          (`self.OpenDoor`)
          (else
            (`/Game/ThirdPerson/Blueprints/BP_ThirdPersonGameMode.Message` (`self.Gamemode`) (`KismetTextLibrary.Conv_StringToText` (`KismetStringLibrary.Concat_StrStr` "You need " (`KismetTextLibrary.Conv_TextToString` (`/Game/Actors/BP_Key.KeyName` (`self.Key`))) " to open this door")) 5.0)))
        (elif (`self.IsValid`)
          (`self.OpenDoor`)
          (else
            (`/Game/ThirdPerson/Blueprints/BP_ThirdPersonGameMode.Message` (`self.Gamemode`) "Does not open from this side" 5.0)))))))

(event `self.Front.OnComponentBeginOverlap`
  (params (OverlappedComponent :type "PrimitiveComponent Object Reference") (OtherActor :type "Actor Object Reference") (OtherComp :type "PrimitiveComponent Object Reference") (OtherBodyIndex :type Integer) (bFromSweep :type Boolean) (SweepResult :type "HitResult Structure (by ref)"))
  (bind _asbp_third_person_character (cast `/Game/ThirdPerson/Blueprints/BP_ThirdPersonCharacter` OtherActor))
  (bind _gamemode (`/Game/ThirdPerson/Blueprints/BP_ThirdPersonCharacter.Gamemode` _asbp_third_person_character))
  (if (`KismetMathLibrary.BooleanNOR` (`NavMovementComponent.IsFalling` (`Character.CharacterMovement` _asbp_third_person_character)) (`/Game/ThirdPerson/Blueprints/BP_ThirdPersonGameMode.PlayerDead` _gamemode))
    (set `self.Inside` true)
    (set `self.IsValid` (`self.CanOpenFront`))
    (`/Game/ThirdPerson/Blueprints/BP_ThirdPersonGameMode.CanInteract` _gamemode)))

(event `self.Front.OnComponentEndOverlap`
  (params (OverlappedComponent :type "PrimitiveComponent Object Reference") (OtherActor :type "Actor Object Reference") (OtherComp :type "PrimitiveComponent Object Reference") (OtherBodyIndex :type Integer))
  (bind _asbp_third_person_character (cast `/Game/ThirdPerson/Blueprints/BP_ThirdPersonCharacter` OtherActor))
  (`/Game/ThirdPerson/Blueprints/BP_ThirdPersonGameMode.CannotInteract` (`/Game/ThirdPerson/Blueprints/BP_ThirdPersonCharacter.Gamemode` _asbp_third_person_character))
  (set `self.Inside` false)
  (set `self.IsValid` false))

(event `self.Back.OnComponentBeginOverlap`
  (params (OverlappedComponent :type "PrimitiveComponent Object Reference") (OtherActor :type "Actor Object Reference") (OtherComp :type "PrimitiveComponent Object Reference") (OtherBodyIndex :type Integer) (bFromSweep :type Boolean) (SweepResult :type "HitResult Structure (by ref)"))
  (bind _asbp_third_person_character (cast `/Game/ThirdPerson/Blueprints/BP_ThirdPersonCharacter` OtherActor))
  (bind _gamemode (`/Game/ThirdPerson/Blueprints/BP_ThirdPersonCharacter.Gamemode` _asbp_third_person_character))
  (if (`KismetMathLibrary.BooleanNOR` (`NavMovementComponent.IsFalling` (`Character.CharacterMovement` _asbp_third_person_character)) (`/Game/ThirdPerson/Blueprints/BP_ThirdPersonGameMode.PlayerDead` _gamemode))
    (set `self.Inside` true)
    (set `self.IsValid` (`self.CanOpenBack`))
    (`/Game/ThirdPerson/Blueprints/BP_ThirdPersonGameMode.CanInteract` _gamemode)))

(event `OpenDoor`
  (`|ExecutionSequence`
    (:`then_0`
      (bind (_direction _value) (`Timeline|Rotation`)
        (:`Update`
          (`SceneComponent.K2_SetRelativeRotation` (`self.Cylinder`) (`KismetMathLibrary.MakeRotator` 0.0 0.0 (* _value 90.0)) false false))))
    (:`then_1`
      (`ActorComponent.K2_DestroyComponent` (`self.Back`))
      (`ActorComponent.K2_DestroyComponent` (`self.Front`)))))

(event `self.Back.OnComponentEndOverlap`
  (params (OverlappedComponent :type "PrimitiveComponent Object Reference") (OtherActor :type "Actor Object Reference") (OtherComp :type "PrimitiveComponent Object Reference") (OtherBodyIndex :type Integer))
  (bind _asbp_third_person_character (cast `/Game/ThirdPerson/Blueprints/BP_ThirdPersonCharacter` OtherActor))
  (`/Game/ThirdPerson/Blueprints/BP_ThirdPersonGameMode.CannotInteract` (`/Game/ThirdPerson/Blueprints/BP_ThirdPersonCharacter.Gamemode` _asbp_third_person_character))
  (set `self.Inside` false)
  (set `self.IsValid` false))

(fn `UserConstructionScript`
  (`SceneComponent.SetHiddenInGame` (`self.FrontText`) (not (`self.VisibleInGame`)) false)
  (`SceneComponent.SetHiddenInGame` (`self.BackText`) (not (`self.VisibleInGame`)) false)
  (`SceneComponent.SetHiddenInGame` (`self.Front`) (not (`self.VisibleInGame`)) false)
  (`SceneComponent.SetHiddenInGame` (`self.Box`) (not (`self.VisibleInGame`)) false)
  (`SceneComponent.SetHiddenInGame` (`self.Back`) (not (`self.VisibleInGame`)) false)
  (if (`self.RequireKey`)
    (`TextRenderComponent.SetTextRenderColor` (`self.BackText`) (make `Color` 255 0 0 255))
    (`TextRenderComponent.SetTextRenderColor` (`self.FrontText`) (make `Color` 255 0 0 255))
    (else
      (`|ExecutionSequence`
        (:`then_0`
          (if (`self.CanOpenBack`)
            (`TextRenderComponent.SetTextRenderColor` (`self.BackText`) (make `Color` 0 255 0 255))
            (else
              (`TextRenderComponent.SetTextRenderColor` (`self.BackText`) (make `Color` 0 0 255 255)))))
        (:`then_1`
          (if (`self.CanOpenFront`)
            (`TextRenderComponent.SetTextRenderColor` (`self.FrontText`) (make `Color` 0 255 0 255))
            (else
              (`TextRenderComponent.SetTextRenderColor` (`self.FrontText`) (make `Color` 0 0 255 255)))))))))