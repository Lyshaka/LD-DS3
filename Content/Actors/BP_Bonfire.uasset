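; Bonfire actor that restores the player's health and registers itself as the game mode's current bonfire.
; Sphere overlap flags the player as near, if alive and not falling, and toggles the game mode's interact state.
; While near, Tick polls the E key through a resettable DoOnce to call Activate.
; The first activation also lights the initially dark material and briefly shows a "bonfire lit" widget.
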(event `self.ReceiveBeginPlay`
  (bind _outactors (`GameplayStatics.GetAllActorsOfClass` "BP_Bonfire_C"))
  (set `self.BonfireList` _outactors)
  (bind _returnvalue (`|CreateWidget` "/Game/Interface/WB_BonfireLit.WB_BonfireLit_C"))
  (set `self.BonfireLit` _returnvalue))

(event `self.ReceiveTick`
  (params (DeltaSeconds :type "Float (single-precision)"))
  (if (`self.Near`)
    (if (`PlayerController.IsInputKeyDown` (`GameplayStatics.GetPlayerController` 0) "E")
      (`/Engine/EditorBlueprintResources/StandardMacros.DoOnce` false :!label _label
        (:`Completed`
          (`self.Activate`)))
      (else
        (goto _label :!via `Reset`)))))

(event `LightFire`
  (`MeshComponent.SetVectorParameterValueOnMaterials` (`self.SM_Bonfire`) "Color" (1.0 0.3 0.0))
  (`MeshComponent.SetScalarParameterValueOnMaterials` (`self.SM_Bonfire`) "Intensity" 0.03))

(event `Activate`
  (`|ExecutionSequence`
    (:`then_0`
      (bind _asbp_third_person_character (cast `/Game/ThirdPerson/Blueprints/BP_ThirdPersonCharacter` (`GameplayStatics.GetPlayerCharacter` 0)))
      (set `/Game/ThirdPerson/Blueprints/BP_ThirdPersonCharacter.HealthPoint` 100.0 _asbp_third_person_character)
      (set `/Game/ThirdPerson/Blueprints/BP_ThirdPersonGameMode.CurrentBonfire` self (`/Game/ThirdPerson/Blueprints/BP_ThirdPersonCharacter.Gamemode` _asbp_third_person_character)))
    (:`then_1`
      (`/Engine/EditorBlueprintResources/StandardMacros.DoOnce` false
        (:`Completed`
          (`self.LightFire`)
          (`UserWidget.AddToViewport` (`self.BonfireLit`) 0)
          (`KismetSystemLibrary.Delay` 3.0)
          (`Widget.RemoveFromParent` (`self.BonfireLit`)))))))

(event `self.Sphere.OnComponentBeginOverlap`
  (params (OverlappedComponent :type "PrimitiveComponent Object Reference") (OtherActor :type "Actor Object Reference") (OtherComp :type "PrimitiveComponent Object Reference") (OtherBodyIndex :type Integer) (bFromSweep :type Boolean) (SweepResult :type "HitResult Structure (by ref)"))
  (bind _asbp_third_person_character (cast `/Game/ThirdPerson/Blueprints/BP_ThirdPersonCharacter` OtherActor))
  (bind _gamemode (`/Game/ThirdPerson/Blueprints/BP_ThirdPersonCharacter.Gamemode` _asbp_third_person_character))
  (`/Engine/EditorBlueprintResources/StandardMacros.IsValid` _gamemode
    (:`Is Valid`
      (if (`KismetMathLibrary.BooleanNOR` (`NavMovementComponent.IsFalling` (`Character.CharacterMovement` _asbp_third_person_character)) (`/Game/ThirdPerson/Blueprints/BP_ThirdPersonGameMode.PlayerDead` _gamemode))
        (set `self.Near` true)
        (`/Game/ThirdPerson/Blueprints/BP_ThirdPersonGameMode.CanInteract` _gamemode)))))

(event `self.Sphere.OnComponentEndOverlap`
  (params (OverlappedComponent :type "PrimitiveComponent Object Reference") (OtherActor :type "Actor Object Reference") (OtherComp :type "PrimitiveComponent Object Reference") (OtherBodyIndex :type Integer))
  (bind _asbp_third_person_character (cast `/Game/ThirdPerson/Blueprints/BP_ThirdPersonCharacter` OtherActor))
  (`/Game/ThirdPerson/Blueprints/BP_ThirdPersonGameMode.CannotInteract` (`/Game/ThirdPerson/Blueprints/BP_ThirdPersonCharacter.Gamemode` _asbp_third_person_character))
  (set `self.Near` false))

(fn `UserConstructionScript`
  (`MeshComponent.SetVectorParameterValueOnMaterials` (`self.SM_Bonfire`) "Color" (0.0 0.0 0.0))
  (`MeshComponent.SetScalarParameterValueOnMaterials` (`self.SM_Bonfire`) "Intensity" 0.0))